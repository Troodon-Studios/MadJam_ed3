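; Fighting board that spawns enemy and player mobs and runs their combat.
; Six spawner events, three per side, create mobs with random data rows, each gated by its own cooldown flag.
; A looping one-second CombatTick moves mobs, damages their objectives, drops the dead from the active list and resumes killers after a delay.
; Overlap volumes stop player mobs at Center and enemy mobs at End.
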(event `Spawner4`
  (bind _canspawn_ (`self.canSpawn?`))
  (if (`|GetArrayItem` _canspawn_ 3)
    (`KismetArrayLibrary.Array_Set` _canspawn_ 3)
    (`self.SpawnPlayerMobActor` (`self.Spawn4`))
    (`KismetSystemLibrary.Delay` (`self.Cooldown`))
    (`KismetArrayLibrary.Array_Set` _canspawn_ 3 true)))

(event `Spawner5`
  (bind _canspawn_ (`self.canSpawn?`))
  (if (`|GetArrayItem` _canspawn_ 4)
    (`KismetArrayLibrary.Array_Set` _canspawn_ 4)
    (`self.SpawnPlayerMobActor` (`self.Spawn5`))
    (`KismetSystemLibrary.Delay` (`self.Cooldown`))
    (`KismetArrayLibrary.Array_Set` _canspawn_ 4 true)))

(event `Spawner1`
  (bind _canspawn_ (`self.canSpawn?`))
  (if (`|GetArrayItem` _canspawn_)
    (`KismetArrayLibrary.Array_Set` _canspawn_)
    (`self.SpawnEnemyMobActor` (`self.Spawn1`))
    (`KismetSystemLibrary.Delay` (`self.Cooldown`))
    (`KismetArrayLibrary.Array_Set` _canspawn_ 0 true)))

(event `Spawner6`
  (bind _canspawn_ (`self.canSpawn?`))
  (if (`|GetArrayItem` _canspawn_ 5)
    (`KismetArrayLibrary.Array_Set` _canspawn_ 5)
    (`self.SpawnPlayerMobActor` (`self.Spawn6`))
    (`KismetSystemLibrary.Delay` (`self.Cooldown`))
    (`KismetArrayLibrary.Array_Set` _canspawn_ 5 true)))

(event `Spawner2`
  (bind _canspawn_ (`self.canSpawn?`))
  (if (`|GetArrayItem` _canspawn_ 1)
    (`KismetArrayLibrary.Array_Set` _canspawn_ 1)
    (`self.SpawnEnemyMobActor` (`self.Spawn2`))
    (`KismetSystemLibrary.Delay` (`self.Cooldown`))
    (`KismetArrayLibrary.Array_Set` _canspawn_ 1 true)))

(event `Spawner 3`
  (bind _canspawn_ (`self.canSpawn?`))
  (if (`|GetArrayItem` _canspawn_ 2)
    (`KismetArrayLibrary.Array_Set` _canspawn_ 2)
    (`self.SpawnEnemyMobActor` (`self.Spawn3`))
    (`KismetSystemLibrary.Delay` (`self.Cooldown`))
    (`KismetArrayLibrary.Array_Set` _canspawn_ 2 true)))

(event `self.ReceiveBeginPlay`
  (`KismetSystemLibrary.K2_SetTimer` null "CombatTick" 1.0 true))

(event `Resumeovement`
  (params (MobActor :type "/Game/Blueprints/Mobs/MobActor Object Reference"))
  (`KismetSystemLibrary.Delay` 1.0)
  (`/Game/Blueprints/Mobs/MobActor.ResumeMovement` MobActor))

(event `self.Center.OnComponentBeginOverlap`
  (params (OverlappedComponent :type "PrimitiveComponent Object Reference") (OtherActor :type "Actor Object Reference") (OtherComp :type "PrimitiveComponent Object Reference") (OtherBodyIndex :type Integer) (bFromSweep :type Boolean) (SweepResult :type "HitResult Structure (by ref)"))
  (bind _asplayer_mob_actor (cast `/Game/Blueprints/Mobs/PlayerMobActor` OtherActor))
  (`/Game/Blueprints/Mobs/MobActor.Stop` _asplayer_mob_actor))

(event `self.End.OnComponentBeginOverlap`
  (params (OverlappedComponent :type "PrimitiveComponent Object Reference") (OtherActor :type "Actor Object Reference") (OtherComp :type "PrimitiveComponent Object Reference") (OtherBodyIndex :type Integer) (bFromSweep :type Boolean) (SweepResult :type "HitResult Structure (by ref)"))
  (bind _asenemy_mob_actor (cast `/Game/Blueprints/Mobs/EnemyMobActor` OtherActor))
  (`/Game/Blueprints/Mobs/MobActor.Stop` _asenemy_mob_actor))

(fn `CombatTick`
  (locals (DeadMobs :type "Array of Object Object Reference") (DeadMobActors :type "Array of /Game/Blueprints/Mobs/MobActor Object Reference"))
  (for _array_element (`self.MobsActors`)
    (if (`/Game/Blueprints/Mobs/MobActor.canMove?` _array_element)
      (`/Game/Blueprints/Mobs/MobActor.Move` _array_element))
    (bind _objective (`/Game/Blueprints/Mobs/MobActor.Objective` _array_element)
      (:`then`
        (`/Game/Blueprints/Mobs/MobActor.AttackAnimation` _array_element)
        (`/Game/Blueprints/Mobs/MobActor.TakeDamage` _objective (`/Game/Blueprints/Mobs/MobActor.Damage` _array_element))
        (if (`/Game/Blueprints/Mobs/MobActor.isDead?` _objective)
          (`KismetArrayLibrary.Array_Add` (`local.DeadMobActors`) _objective)
          (set `/Game/Blueprints/Mobs/MobActor.Objective` null _array_element)
          (`self.Resumeovement` _array_element)))
      (:`else`)))
  (for _array_element_2 (`local.DeadMobActors`)
    (`KismetArrayLibrary.Array_RemoveItem` (`self.MobsActors`) _array_element_2)))

(fn `SpawnEnemyMobActor`
  (params (Spawner :type "SceneComponent Object Reference"))
  (bind _returnvalue (`SceneComponent.K2_GetComponentToWorld` Spawner))
  (bind _returnvalue_2 (`|SpawnActorFromClass` "/Game/Blueprints/Mobs/EnemyMobActor.EnemyMobActor_C" (`KismetMathLibrary.MakeTransform` (`KismetMathLibrary.MakeVector` (.x (.location _returnvalue)) (.y (.location _returnvalue)) (.z (.location _returnvalue))) (.rotation _returnvalue) (.scale _returnvalue)) "Undefined" "MultiplyWithRoot" null (struct) null))
  (set `/Game/Blueprints/Mobs/MobActor.RowName` (`|GetArrayItem` (`self.Names`) (`KismetMathLibrary.RandomInteger` 3)) _returnvalue_2)
  (`/Game/Blueprints/Mobs/MobActor.ChangeMob` _returnvalue_2)
  (`KismetArrayLibrary.Array_Add` (`self.MobsActors`) _returnvalue_2))

(fn `SpawnPlayerMobActor`
  (params (Spawner :type "SceneComponent Object Reference"))
  (bind _returnvalue (`SceneComponent.K2_GetComponentToWorld` Spawner))
  (bind _returnvalue_2 (`|SpawnActorFromClass` "/Game/Blueprints/Mobs/PlayerMobActor.PlayerMobActor_C" (`KismetMathLibrary.MakeTransform` (`KismetMathLibrary.MakeVector` (.x (.location _returnvalue)) (.y (.location _returnvalue)) (.z (.location _returnvalue))) (.rotation _returnvalue) (.scale _returnvalue)) "Undefined" "MultiplyWithRoot" null (struct) null))
  (set `/Game/Blueprints/Mobs/MobActor.RowName` (`|GetArrayItem` (`self.Names`) (`KismetMathLibrary.RandomIntegerInRange` 3 8)) _returnvalue_2)
  (`/Game/Blueprints/Mobs/MobActor.ChangeMob` _returnvalue_2)
  (`KismetArrayLibrary.Array_Add` (`self.MobsActors`) _returnvalue_2))

(fn `UserConstructionScript`)