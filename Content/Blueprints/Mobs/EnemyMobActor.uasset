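; EnemyMobActor is the enemy-side mob, using its AttackRange component to decide when to halt and what to target.
; A PlayerMobActor entering range pauses movement and becomes the Objective, while another EnemyMobActor entering range only pauses movement.
; Movement resumes only when an EnemyMobActor leaves range; a player mob leaving triggers no action here.
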(event `self.AttackRange.OnComponentBeginOverlap`
  (params (OverlappedComponent :type "PrimitiveComponent Object Reference") (OtherActor :type "Actor Object Reference") (OtherComp :type "PrimitiveComponent Object Reference") (OtherBodyIndex :type Integer) (bFromSweep :type Boolean) (SweepResult :type "HitResult Structure (by ref)"))
  (bind _asmob_actor (cast `/Game/Blueprints/Mobs/MobActor` OtherActor))
  (cast `/Game/Blueprints/Mobs/PlayerMobActor` OtherActor
    (:`then`
      (`self.PauseMovement`)
      (set `self.Objective` _asmob_actor))
    (:`CastFailed`
      (cast `/Game/Blueprints/Mobs/EnemyMobActor` OtherActor)
      (`self.PauseMovement`))))

(event `self.AttackRange.OnComponentEndOverlap`
  (params (OverlappedComponent :type "PrimitiveComponent Object Reference") (OtherActor :type "Actor Object Reference") (OtherComp :type "PrimitiveComponent Object Reference") (OtherBodyIndex :type Integer))
  (cast `/Game/Blueprints/Mobs/EnemyMobActor` OtherActor)
  (`self.ResumeMovement`))

(fn `UserConstructionScript`
  (`parent.UserConstructionScript`))