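; Mob Blueprint for a walking enemy or creature with health, a death state and a timed removal.
; Tick drives it along its capsule's forward vector while CanWalk is set, and re-enables walking after a delay once Objective is invalid.
; TakeDamage subtracts health or calls Death, which disables collision and starts DeathVanish.
; The Vanish timeline nudges the actor upward, then clears Objective and destroys it after a delay.
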(event `self.ReceiveTick`
  (params (DeltaSeconds :type "Float (single-precision)"))
  (if (`self.canWalk?`)
    (`self.AddMovementInput` (`SceneComponent.GetForwardVector` (`self.CapsuleComponent`)))
    (else
      (`self.Objective`
        (:`then`)
        (:`else`
          (`KismetSystemLibrary.Delay` 1.0)
          (set `self.canWalk?` true))))))

(event `DeathVanish`
  (bind (_returnvalue_x _returnvalue_y _returnvalue_z) (`KismetMathLibrary.BreakVector` (`SceneComponent.K2_GetComponentLocation` (`self.CapsuleComponent`))))
  (bind (_direction _pos) (`Timeline|Vanish` :!via `PlayFromStart`)
    (:`Update`
      (`self.K2_SetActorLocation` (`KismetMathLibrary.MakeVector` _returnvalue_x _returnvalue_y (`KismetMathLibrary.Lerp` _returnvalue_z (+ _returnvalue_z 10.0) _pos))))
    (:`Finished`
      (set `self.Objective` null)
      (`KismetSystemLibrary.Delay` 5.0)
      (`self.K2_DestroyActor`))))

(fn `Death`
  (`PrimitiveComponent.SetCollisionEnabled` (`self.CapsuleComponent`) "NoCollision")
  (`self.DeathVanish`)
  (set `self.isDead?` true))

(fn `TakeDamage`
  (params (Damage :type Integer))
  (bind _returnvalue (- (`self.Health`) Damage))
  (if (<= _returnvalue 0)
    (`self.Death`)
    (else
      (set `self.Health` _returnvalue))))

(fn `UserConstructionScript`)