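; Mob actor that moves along its mesh's forward vector, takes damage and vanishes on death.
; BeginPlay starts a looping timer, while Move teleports the actor by Speed when CanMove allows; separate functions stop, pause or resume movement.
; Lethal damage triggers a timeline that nudges the actor upward, then clears Objective and destroys it after a delay.
; ChangeMob applies mesh, rotation and scale from a data table row.
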(event `self.ReceiveBeginPlay`
  (`KismetSystemLibrary.K2_SetTimerDelegate` :`Time` 1.0 :`bLooping` true))

(event `Move`
  (if (`self.canMove?`)
    (`self.K2_AddActorWorldOffset` (* (`SceneComponent.GetForwardVector` (`self.SkeletalMesh`)) (`self.Speed`)) false true)))

(event `DeathVanish`
  (bind (_returnvalue_x _returnvalue_y _returnvalue_z) (`KismetMathLibrary.BreakVector` (`SceneComponent.K2_GetComponentLocation` (`self.Box`))))
  (bind (_direction _pos) (`Timeline|Timeline` :!via `PlayFromStart`)
    (:`Update`
      (`self.K2_SetActorRelativeLocation` (`KismetMathLibrary.MakeVector` _returnvalue_x _returnvalue_y (`KismetMathLibrary.Lerp` _returnvalue_z (+ _returnvalue_z 2.0) _pos))))
    (:`Finished`
      (set `self.Objective` null)
      (`KismetSystemLibrary.Delay` 5.0)
      (`self.K2_DestroyActor`))))

(event `self.ReceiveTick`
  (params (DeltaSeconds :type "Float (single-precision)")))

(fn `ChangeMob`
  (bind _skeletalmesh (`self.SkeletalMesh`))
  (bind _returnvalue (`|GetDataTableRow` (break `DataTableRowHandle` (break `/Game/Blueprints/Mobs/S_Slots` (`self.MobData`))) (`self.RowName`))
    (:`then`
      (bind (_health _damage _speed _skeletalmesh_2 _scale _rotation) (break `/Game/Blueprints/Mobs/S_Mobs` _returnvalue))
      (`SkeletalMeshComponent.SetSkeletalMeshAsset` _skeletalmesh _skeletalmesh_2)
      (`SceneComponent.K2_AddRelativeRotation` _skeletalmesh _rotation false false)
      (`SceneComponent.SetRelativeScale3D` _skeletalmesh (* (`SceneComponent.RelativeScale3D` _skeletalmesh) _scale)))))

(fn `Death`)

(fn `PauseMovement`
  (set `self.Speed` 0.0))

(fn `ResumeMovement`
  (set `self.Speed` 1.0))

(fn `Stop`
  (set `self.canMove?` false))

(fn `TakeDamage`
  (params (Damage :type Integer))
  (bind _returnvalue (- (`self.Health`) Damage))
  (if (<= _returnvalue 0)
    (set `self.isDead?` true)
    (`self.DeathVanish`)
    (else
      (set `self.Health` _returnvalue))))

(fn `UserConstructionScript`)