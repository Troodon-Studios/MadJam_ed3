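; PlayerMob is a player-side mob Blueprint that reacts to what overlaps its Box component.
; On overlap with any Mob other than its owner, it stops walking via CanWalk and, if that Mob is an EnemyMob, sets it as its Objective.
; On overlap with a FightingBoard instead, it sets its max walk speed to zero.
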(event `self.Box.OnComponentBeginOverlap`
  (params (OverlappedComponent :type "PrimitiveComponent Object Reference") (OtherActor :type "Actor Object Reference") (OtherComp :type "PrimitiveComponent Object Reference") (OtherBodyIndex :type Integer) (bFromSweep :type Boolean) (SweepResult :type "HitResult Structure (by ref)"))
  (if (!= OtherActor (`self.GetOwner`))
    (bind _asmob (cast `/Game/Blueprints/Mobs/Mob` OtherActor)
      (:`then`
        (set `self.canWalk?` false)
        (cast `/Game/Blueprints/Mobs/EnemyMob` _asmob)
        (set `self.Objective` _asmob))
      (:`CastFailed`
        (cast `/Game/Blueprints/Modules/FightingBoard` OtherActor)
        (set `CharacterMovementComponent.MaxWalkSpeed` 0.0 (`self.CharacterMovement`))))))

(fn `UserConstructionScript`
  (`parent.UserConstructionScript`))