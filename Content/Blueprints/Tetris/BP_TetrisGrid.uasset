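; Tetris grid actor that recognizes colored block patterns and unlocks monsters on the player.
; RefreshArray uses overlaps with row and column line boxes to position each BP_SingleBlock in a flattened array indexed by NCols.
; It then runs six hard-coded shape matchers, mostly chained Check calls stepping between neighboring cells by color.
; A match destroys the arrayed blocks and calls ActivateMonster on the first BP_Player.
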(event `self.ReceiveBeginPlay`
  (`self.SetupLines`))

(fn `Beast_1`
  (params (First :type Integer))
  (locals (NewLocalVar :type Integer))
  (bind _returnvalue (+ First (`self.N_cols`)))
  (bind _output (`|GetArrayItem` (`self.BlocksArray`) _returnvalue))
  (bind _returnvalue_2 (+ _returnvalue 1))
  (bind _output_2 (`|GetArrayItem` (`self.BlocksArray`) _returnvalue_2))
  (bind _returnvalue_3 (+ _returnvalue_2 1))
  (bind _output_3 (`|GetArrayItem` (`self.BlocksArray`) _returnvalue_3))
  (bind _returnvalue_4 (+ _returnvalue_3 (`self.N_cols`)))
  (bind _returnvalue_5 (+ _returnvalue_3 1))
  (bind _output_4 (`|GetArrayItem` (`self.BlocksArray`) _returnvalue_4))
  (bind _output_5 (`|GetArrayItem` (`self.BlocksArray`) _returnvalue_5))
  (bind _returnvalue_6 (+ _returnvalue_4 (`self.N_cols`)))
  (bind _returnvalue_7 (+ _returnvalue_5 1))
  (bind _output_6 (`|GetArrayItem` (`self.BlocksArray`) _returnvalue_6))
  (bind _output_7 (`|GetArrayItem` (`self.BlocksArray`) _returnvalue_7))
  (bind _returnvalue_8 (+ _returnvalue_7 1))
  (bind _returnvalue_9 (+ _returnvalue_6 1))
  (bind _output_8 (`|GetArrayItem` (`self.BlocksArray`) _returnvalue_8))
  (bind _output_9 (`|GetArrayItem` (`self.BlocksArray`) _returnvalue_9))
  (bind _output_10 (`|GetArrayItem` (`self.BlocksArray`) (- _returnvalue_9 (`self.N_cols`))))
  (bind _output_11 (`|GetArrayItem` (`self.BlocksArray`) (- _returnvalue_8 (`self.N_cols`))))
  (if (`KismetSystemLibrary.IsValid` _output)
    (if (== (`/Game/Blueprints/Tetris/BP_SingleBlock.colorType` _output) 2)
      (if (`KismetSystemLibrary.IsValid` _output_2)
        (if (== (`/Game/Blueprints/Tetris/BP_SingleBlock.colorType` _output_2) 2)
          (if (`KismetSystemLibrary.IsValid` _output_3)
            (if (== (`/Game/Blueprints/Tetris/BP_SingleBlock.colorType` _output_3) 2)
              (`|ExecutionSequence`
                (:`then_0`
                  (if (`KismetSystemLibrary.IsValid` _output_4)
                    (if (== (`/Game/Blueprints/Tetris/BP_SingleBlock.colorType` _output_4) 3)
                      (if (`KismetSystemLibrary.IsValid` _output_6)
                        (if (== (`/Game/Blueprints/Tetris/BP_SingleBlock.colorType` _output_6) 3)
                          (if (`KismetSystemLibrary.IsValid` _output_9)
                            (if (== (`/Game/Blueprints/Tetris/BP_SingleBlock.colorType` _output_9) 3)
                              (if (`KismetSystemLibrary.IsValid` _output_10)
                                _))))))))
                (:`then_1`
                  (if (`KismetSystemLibrary.IsValid` _output_5)
                    (if (== (`/Game/Blueprints/Tetris/BP_SingleBlock.colorType` _output_5) 2)
                      (if (`KismetSystemLibrary.IsValid` _output_7)
                        (if (== (`/Game/Blueprints/Tetris/BP_SingleBlock.colorType` _output_7) 2)
                          (if (`KismetSystemLibrary.IsValid` _output_8)
                            (if (== (`/Game/Blueprints/Tetris/BP_SingleBlock.colorType` _output_8) 2)
                              (if (`KismetSystemLibrary.IsValid` _output_11)
                                (if (and (== (`/Game/Blueprints/Tetris/BP_SingleBlock.colorType` _output_10) 3) (== (`/Game/Blueprints/Tetris/BP_SingleBlock.colorType` _output_11) 2))
                                  (`KismetSystemLibrary.PrintString` "Monstro 1")
                                  (`self.UnlockBeast` 5))))))))))))))))))

(fn `Beast_2`
  (params (Index :type Integer))
  (bind _resultante (`self.Check` Index (`self.N_cols`) 2))
  (bind _resultante_2 (`self.Check` _resultante 1 2))
  (bind _resultante_3 (`self.Check` _resultante_2 1 2))
  (bind _resultante_4 (`self.Check` _resultante_3 1 1))
  (`|ExecutionSequence`
    (:`then_0`
      (bind _resultante_5 (`self.Check` _resultante_4 (`self.N_cols`) 1))
      (bind _resultante_6 (`self.Check` _resultante_5 (`self.N_cols`) 1))
      (bind _resultante_7 (`self.Check` _resultante_6 (`self.N_cols`) 5))
      (bind _resultante_8 (`self.Check` _resultante_7 (`self.N_cols`) 5))
      (`|ExecutionSequence`
        (:`then_0`
          (bind (_resultante_9 _valid) (`self.Check` _resultante_8 -1 5)))
        (:`then_1`
          (bind (_resultante_10 _valid_2) (`self.Check` _resultante_8 1 5)))))
    (:`then_1`
      (bind _resultante_11 (`self.Check` _resultante_4 1 2))
      (bind _resultante_12 (`self.Check` _resultante_11 1 2))
      (bind _resultante_13 (`self.Check` _resultante_12 1 2))
      (bind (_resultante_14 _valid_3) (`self.Check` _resultante_13 (* (`self.N_cols`) -1) 2)))
    (:`then_2`
      (bind (_resultante_15 _valid_4) (`self.Check` _resultante_4 (* (`self.N_cols`) -1) 1))
      (if (and _valid _valid_2 _valid_3 _valid_4)
        (`KismetSystemLibrary.PrintString` "Monstro_2")
        (`self.UnlockBeast` 4)))))

(fn `Beast_3`
  (params (Intex :type Integer))
  (bind _resultante (`self.Check` Intex (`self.N_cols`) 5))
  (`|ExecutionSequence`
    (:`then_0`
      (bind _resultante_2 (`self.Check` _resultante (`self.N_cols`) 5))
      (bind _resultante_3 (`self.Check` _resultante_2 (`self.N_cols`) 4))
      (bind (_resultante_4 _valid) (`self.Check` _resultante_3 (`self.N_cols`) 4)))
    (:`then_1`
      (bind _resultante_5 (`self.Check` _resultante 1 5))
      (`|ExecutionSequence`
        (:`then_0`
          (bind _resultante_6 (`self.Check` _resultante_5 (`self.N_cols`) 4))
          (bind (_resultante_7 _valid_2) (`self.Check` _resultante_6 (`self.N_cols`) 4)))
        (:`then_1`
          (bind _resultante_8 (`self.Check` _resultante_5 1 5))
          (`|ExecutionSequence`
            (:`then_0`
              (bind _resultante_9 (`self.Check` _resultante_8 (`self.N_cols`) 4))
              (bind (_resultante_10 _valid_3) (`self.Check` _resultante_9 (`self.N_cols`) 3)))
            (:`then_1`
              (bind _resultante_11 (`self.Check` _resultante_8 1 5))
              (`|ExecutionSequence`
                (:`then_0`
                  (bind _resultante_12 (`self.Check` _resultante_11 (`self.N_cols`) 5))
                  (bind _resultante_13 (`self.Check` _resultante_12 (`self.N_cols`) 4))
                  (bind (_resultante_14 _valid_4) (`self.Check` _resultante_13 (`self.N_cols`) 4)))
                (:`then_1`
                  (bind (_resultante_15 _valid_5) (`self.Check` _resultante_11 (* (`self.N_cols`) -1) 5))
                  (if (and _valid _valid_2 _valid_3 _valid_4 _valid_5)
                    (`KismetSystemLibrary.PrintString` "Monstro 3")
                    (`self.UnlockBeast` 6)))))))))))

(fn `Beast_4`
  (params (Intex :type Integer))
  (bind _resultante (`self.Check` Intex (`self.N_cols`) 2))
  (bind _resultante_2 (`self.Check` _resultante 1 2))
  (bind _resultante_3 (`self.Check` _resultante_2 1 2))
  (bind _resultante_4 (`self.Check` _resultante_3 1 1))
  (`|ExecutionSequence`
    (:`then_0`
      (bind _resultante_5 (`self.Check` _resultante_4 (`self.N_cols`) 1))
      (bind _resultante_6 (`self.Check` _resultante_5 (`self.N_cols`) 1))
      (bind _resultante_7 (`self.Check` _resultante_6 (`self.N_cols`) 5))
      (bind _resultante_8 (`self.Check` _resultante_7 1 5))
      (`|ExecutionSequence`
        (:`then_0`
          (bind (_resultante_9 _valid) (`self.Check` _resultante_8 (`self.N_cols`) 5)))
        (:`then_1`
          (bind (_resultante_10 _valid_2) (`self.Check` _resultante_8 1 5)))))
    (:`then_1`
      (bind (_resultante_11 _valid_3) (`self.Check` _resultante_4 (* (`self.N_cols`) -1) 1))
      (if (and _valid _valid_2 _valid_3)
        (`KismetSystemLibrary.PrintString` "Monstro 4")
        (`self.UnlockBeast` 1)))))

(fn `Beast_5`
  (params (Intex :type Integer))
  (bind _n_cols (`self.N_cols`))
  (bind _n_cols_2 (`self.N_cols`))
  (bind _resultante (`self.Check` Intex 1 4))
  (bind _resultante_2 (`self.Check` _resultante (`self.N_cols`) 4))
  (bind _resultante_3 (`self.Check` _resultante_2 1 4))
  (`|ExecutionSequence`
    (:`then_0`
      (bind _resultante_4 (`self.Check` _resultante_3 (`self.N_cols`) 3))
      (bind _resultante_5 (`self.Check` _resultante_4 (`self.N_cols`) 3))
      (bind _resultante_6 (`self.Check` _resultante_5 (`self.N_cols`) 5))
      (bind _resultante_7 (`self.Check` _resultante_6 -1 5))
      (`|ExecutionSequence`
        (:`then_0`
          (bind (_resultante_8 _valid) (`self.Check` _resultante_7 _n_cols 5)))
        (:`then_1`
          (bind (_resultante_9 _valid_2) (`self.Check` _resultante_7 (* _n_cols -1) 5)))))
    (:`then_1`
      (bind _resultante_10 (`self.Check` _resultante_3 1 4))
      (`|ExecutionSequence`
        (:`then_0`
          (bind _resultante_11 (`self.Check` _resultante_10 (`self.N_cols`) 3))
          (bind _resultante_12 (`self.Check` _resultante_11 (`self.N_cols`) 3))
          (bind _resultante_13 (`self.Check` _resultante_12 (`self.N_cols`) 5))
          (bind _resultante_14 (`self.Check` _resultante_13 1 5))
          (`|ExecutionSequence`
            (:`then_0`
              (bind (_resultante_15 _valid_3) (`self.Check` _resultante_14 _n_cols_2 5)))
            (:`then_1`
              (bind (_resultante_16 _valid_4) (`self.Check` _resultante_14 (* _n_cols_2 -1) 5)))))
        (:`then_1`
          (bind _resultante_17 (`self.Check` _resultante_10 1 4))
          (bind _resultante_18 (`self.Check` _resultante_17 (* (`self.N_cols`) -1) 4))
          (bind (_resultante_19 _valid_5) (`self.Check` _resultante_18 1 4))
          (if (and _valid _valid_2 _valid_3 _valid_4 _valid_5)
            (`KismetSystemLibrary.PrintString` "Monstro 5")
            (`self.UnlockBeast` 2)))))))

(fn `Check`
  (params (Intex :type Integer) (Plus :type Integer) (Raza :type Integer))
  (returns (Resultante :type Integer) (Valid :type Boolean))
  (bind _returnvalue (+ Intex Plus))
  (bind _output (`|GetArrayItem` (`self.BlocksArray`) _returnvalue))
  (bind _returnvalue_2 (== (`/Game/Blueprints/Tetris/BP_SingleBlock.colorType` _output) Raza))
  (if (`KismetSystemLibrary.IsValid` _output)
    (if _returnvalue_2
      (return _returnvalue _returnvalue_2))))

(fn `Monstro_6`
  (params (Intex :type Integer))
  (bind _returnvalue (* (`self.N_cols`) -1))
  (bind _resultante (`self.Check` Intex (`self.N_cols`) 4))
  (bind _resultante_2 (`self.Check` _resultante 1 4))
  (bind _resultante_3 (`self.Check` _resultante_2 (`self.N_cols`) 4))
  (bind _resultante_4 (`self.Check` _resultante_3 (`self.N_cols`) 3))
  (bind _resultante_5 (`self.Check` _resultante_4 (`self.N_cols`) 3))
  (bind _resultante_6 (`self.Check` _resultante_5 1 3))
  (bind _resultante_7 (`self.Check` _resultante_6 _returnvalue 3))
  (bind _resultante_8 (`self.Check` _resultante_7 _returnvalue 4))
  (bind _resultante_9 (`self.Check` _resultante_8 _returnvalue 4))
  (bind _resultante_10 (`self.Check` _resultante_9 1 4))
  (bind (_resultante_11 _valid) (`self.Check` _resultante_10 _returnvalue 4))
  (if _valid
    (`KismetSystemLibrary.PrintString` "Monstro 6")
    (`self.UnlockBeast` 3)))

(fn `RefreshArray`
  (`KismetArrayLibrary.Array_Clear` (`self.BlocksArray`))
  (for (_array_element _array_index) (`self.HorizontalLines`)
    (for _array_element_2 (`PrimitiveComponent.GetOverlappingActors` _array_element "/Game/Blueprints/Tetris/BP_SingleBlock.BP_SingleBlock_C")
      (bind _asbp_single_block (cast `/Game/Blueprints/Tetris/BP_SingleBlock` _array_element_2))
      (bind (_arraypos_x _arraypos_y) (`KismetMathLibrary.BreakVector2D` (`/Game/Blueprints/Tetris/BP_SingleBlock.ArrayPos` _asbp_single_block)))
      (set `/Game/Blueprints/Tetris/BP_SingleBlock.ArrayPos` (`KismetMathLibrary.MakeVector2D` (`KismetMathLibrary.Conv_IntToDouble` _array_index) _arraypos_y) _asbp_single_block)))
  (for (_array_element_3 _array_index_2) (`self.VerticalLines`)
    (for _array_element_4 (`PrimitiveComponent.GetOverlappingActors` _array_element_3 "/Game/Blueprints/Tetris/BP_SingleBlock.BP_SingleBlock_C")
      (bind _asbp_single_block_2 (cast `/Game/Blueprints/Tetris/BP_SingleBlock` _array_element_4))
      (bind _arraypos_x_2 (`KismetMathLibrary.BreakVector2D` (`/Game/Blueprints/Tetris/BP_SingleBlock.ArrayPos` _asbp_single_block_2)))
      (set `/Game/Blueprints/Tetris/BP_SingleBlock.ArrayPos` (`KismetMathLibrary.MakeVector2D` _arraypos_x_2 (`KismetMathLibrary.Conv_IntToDouble` _array_index_2)) _asbp_single_block_2)))
  (bind _outactors (`GameplayStatics.GetAllActorsOfClass` "/Game/Blueprints/Tetris/BP_SingleBlock.BP_SingleBlock_C"))
  (for _array_element_5 _outactors
    (bind (_arraypos_x_3 _arraypos_y_2) (`KismetMathLibrary.BreakVector2D` (`/Game/Blueprints/Tetris/BP_SingleBlock.ArrayPos` _array_element_5)))
    (`KismetArrayLibrary.Array_Set` (`self.BlocksArray`) (`KismetMathLibrary.FTrunc` (+ _arraypos_y_2 (* _arraypos_x_3 (`self.N_cols`)))) _array_element_5 true))
  (for (_array_element_6 _array_index_3) (`self.BlocksArray`)
    (if (`KismetSystemLibrary.IsValid` _array_element_6)
      (switch `int` (`/Game/Blueprints/Tetris/BP_SingleBlock.colorType` _array_element_6)
        (:`2`
          (`|ExecutionSequence`
            (:`then_0`
              (`self.Beast_1` _array_index_3))
            (:`then_1`
              (`self.Beast_2` _array_index_3))
            (:`then_2`
              (`self.Beast_4` _array_index_3))))
        (:`4`
          (`|ExecutionSequence`
            (:`then_0`
              (`self.Beast_5` _array_index_3))
            (:`then_1`
              (`self.Monstro_6` _array_index_3))))
        (:`5`
          (`self.Beast_3` _array_index_3))))))

(fn `SetupLines`
  (set `self.HorizontalLines` (`|MakeArray` (`self.Box18`) (`self.Box17`) (`self.Box16`) (`self.Box15`) (`self.Box14`) (`self.Box19`) (`self.Box13`) (`self.Box25`) (`self.Box24`) (`self.Box23`) (`self.Box22`) (`self.Box21`) (`self.Box20`)))
  (set `self.VerticalLines` (`|MakeArray` (`self.Box12`) (`self.Box11`) (`self.Box10`) (`self.Box9`) (`self.Box8`) (`self.Box7`) (`self.Box6`) (`self.Box5`) (`self.Box4`) (`self.Box3`) (`self.Box2`) (`self.Box1`) (`self.Box`))))

(fn `UnlockBeast`
  (params (int :type Integer))
  (bind _blocksarray (`self.BlocksArray`))
  (for _array_element _blocksarray
    (`self.K2_DestroyActor` _array_element))
  (`KismetArrayLibrary.Array_Clear` _blocksarray)
  (bind _outactors (`GameplayStatics.GetAllActorsOfClass` "/Game/Blueprints/Player/BP_Player.BP_Player_C"))
  (`/Game/Blueprints/Player/BP_Player.ActivateMonster` (`|GetArrayItem` _outactors) int))

(fn `UserConstructionScript`)