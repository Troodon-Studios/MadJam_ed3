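; Tetris line-clearing actor that finds full rows of BP_SingleBlock actors and removes them.
; Each of its box components acts as a row sensor, counting as full at eleven or more overlapping blocks.
; CheckLines destroys those blocks with particle effects, lowers TargetZ on blocks above the cutoff and calls itself recursively.
; CheckBlocksArray then invalidates and greys out blocks whose piece array lacks exactly three valid entries.
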(event `self.ReceiveBeginPlay`)

(fn `CheckBlocksArray`
  (params (block :type "/Game/Blueprints/Tetris/BP_SingleBlock Object Reference"))
  (locals (validLenght :type Integer))
  (bind _firstblock (`/Game/Blueprints/Tetris/BP_SingleBlock.FirstBlock` block))
  (for _array_element (`/Game/Blueprints/Tetris/BP_SingleBlock.BlocksArray` (select `bool` (`KismetSystemLibrary.IsValid` _firstblock) :`false` block :`true` _firstblock))
    (if (`KismetSystemLibrary.IsValid` _array_element)
      (set `local.validLenght` (+ (`local.validLenght`) 1))))
  (bind _output_get (set `/Game/Blueprints/Tetris/BP_SingleBlock.isValid?` (== (`local.validLenght`) 3) block))
  (if (not _output_get)
    (bind _output_get_2 (set `/Game/Blueprints/Tetris/BP_SingleBlock.BlockColor` (struct :`R` 0.145833 :`G` 0.145833 :`B` 0.145833 :`A` 1.0) block))
    (`MeshComponent.SetVectorParameterValueOnMaterials` (`/Game/Blueprints/Tetris/BP_SingleBlock.Cube_1` block) "Color" (`KismetMathLibrary.Conv_LinearColorToVector` _output_get_2))))

(fn `CheckLines`
  (locals (OverlapActors :type "Array of Actor Object Reference") (DropAmount :type "Float (double-precision)") (CuttoffLineZ :type "Float (double-precision)" :default 10000.0))
  (for _array_element (`self.K2_GetComponentsByClass` "/Script/Engine.BoxComponent")
    (bind _output_get (set `local.OverlapActors` (`PrimitiveComponent.GetOverlappingActors` _array_element "/Game/Blueprints/Tetris/BP_SingleBlock.BP_SingleBlock_C")))
    (if (>= (`KismetArrayLibrary.Array_Length` _output_get) 11)
      (set `local.DropAmount` (+ (`local.DropAmount`) 114.5))
      (bind (_returnvalue_x _returnvalue_y _returnvalue_z) (`KismetMathLibrary.BreakVector` (`SceneComponent.K2_GetComponentLocation` _array_element)))
      (if (< _returnvalue_z (`local.CuttoffLineZ`))
        (set `local.CuttoffLineZ` _returnvalue_z)
        (for _array_element_2 (`local.OverlapActors`)
          (`GameplayStatics.SpawnEmitterAtLocation` null (`self.K2_GetActorLocation` _array_element_2))
          (`self.K2_DestroyActor` _array_element_2)
          (bind _outactors (`GameplayStatics.GetAllActorsOfClass` "/Game/Blueprints/Tetris/BP_SingleBlock.BP_SingleBlock_C"))
          (for _array_element_3 _outactors
            (bind (_returnvalue_x_2 _returnvalue_y_2 _returnvalue_z_2) (`KismetMathLibrary.BreakVector` (`self.K2_GetActorLocation` _array_element_3)))
            (if (> _returnvalue_z_2 (`local.CuttoffLineZ`))
              (set `/Game/Blueprints/Tetris/BP_SingleBlock.TargetZ` (- (`/Game/Blueprints/Tetris/BP_SingleBlock.TargetZ` _array_element_3) (`local.DropAmount`)) _array_element_3)))
          (set `local.DropAmount` 0.0)
          (`self.CheckLines`)
          (bind _outactors_2 (`GameplayStatics.GetAllActorsOfClass` "/Game/Blueprints/Tetris/BP_SingleBlock.BP_SingleBlock_C"))
          (for _array_element_4 _outactors_2
            (if (`/Game/Blueprints/Tetris/BP_SingleBlock.isValid?` _array_element_4)
              (`self.CheckBlocksArray` _array_element_4))))))))

(fn `UserConstructionScript`)