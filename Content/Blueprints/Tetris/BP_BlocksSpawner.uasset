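; Tetris spawner that spawns one of seven random tetromino actors at its start location on BeginPlay, passing itself as Spawner.
; Only two Spawn branches then check lines and refresh the grid.
; BreakBlock replaces the active piece with single blocks, registering them on the first one.
; TryLateralMovement reverts moves that overlap WorldStatic, but its calls, like the rotation and speed-up logic, sit on unconnected nodes, as does the ActualBlock assignment.
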(event `InputAction|RotateBlock`
  (params (Key :type "Key Structure")))

(event `InputAction|MoveLeft`
  (params (Key :type "Key Structure")))

(event `InputAction|MoveRight`
  (params (Key :type "Key Structure")))

(event `InputAction|SpeedUp`
  (params (Key :type "Key Structure")))

(event `self.ReceiveBeginPlay`
  (set `self.StartPos` (`self.K2_GetActorLocation`))
  (`self.Spawn`))

(fn `BreakBlock`
  (bind _actualblock (`self.ActualBlock`))
  (bind _firstblock (`self.FirstBlock`))
  (for _array_element (`SceneComponent.GetChildrenComponents` (`/Game/Blueprints/Tetris/BP_FallingBlock.DefaultSceneRoot` (`self.ActualBlock`)) false)
    (bind (_returnvalue_location _returnvalue_rotation) (`KismetMathLibrary.BreakTransform` (`SceneComponent.K2_GetComponentToWorld` _array_element)))
    (bind _returnvalue (`|SpawnActorFromClass` "/Game/Blueprints/Tetris/BP_SingleBlock.BP_SingleBlock_C" (`KismetMathLibrary.MakeTransform` _returnvalue_location _returnvalue_rotation) "Undefined" "MultiplyWithRoot" null (`/Game/Blueprints/Tetris/BP_FallingBlock.Color` _actualblock) (`self.GetTransform` _actualblock) 0 null))
    (if (`KismetSystemLibrary.IsValid` _firstblock)
      (`KismetArrayLibrary.Array_Add` (`/Game/Blueprints/Tetris/BP_SingleBlock.BlocksArray` _firstblock) _returnvalue)
      (set `/Game/Blueprints/Tetris/BP_SingleBlock.FirstBlock` _firstblock _returnvalue)
      (else
        (`/Engine/EditorBlueprintResources/StandardMacros.DoOnce` false
          (:`Completed`
            (set `self.FirstBlock` _returnvalue))))))
  (`self.K2_DestroyActor` (`self.ActualBlock`))
  (set `self.ActualBlock` null))

(fn `Spawn`
  (bind _returnvalue (`self.GetActorScale3D`))
  (bind _startpos (`self.StartPos`))
  (switch `int` (`KismetMathLibrary.RandomIntegerInRange` 0 6)
    (:`0`
      (`|SpawnActorFromClass` "/Game/Blueprints/Tetris/Types/BC_BlockGreen.BC_BlockGreen_C" (`KismetMathLibrary.MakeTransform` _startpos (struct) _returnvalue) "Undefined" "MultiplyWithRoot" null (struct) self null)
      (`/Game/Blueprints/Tetris/BP_CheckLines.CheckLines` (`self.CheckLineActors`) :!label _label)
      (`/Game/Blueprints/Tetris/BP_TetrisGrid.RefreshArray` (`self.TetrisGrid`)))
    (:`1`
      (`|SpawnActorFromClass` "/Game/Blueprints/Tetris/Types/BC_BlockYellow.BC_BlockYellow_C" (`KismetMathLibrary.MakeTransform` _startpos (struct) _returnvalue) "Undefined" "MultiplyWithRoot" null (struct) self null)
      (goto _label))
    (:`2`
      (`|SpawnActorFromClass` "/Game/Blueprints/Tetris/Types/BC_BlockGreen_i.BC_BlockGreen_i_C" (`KismetMathLibrary.MakeTransform` _startpos (struct) _returnvalue) "Undefined" "MultiplyWithRoot" null (struct) self null))
    (:`3`
      (`|SpawnActorFromClass` "/Game/Blueprints/Tetris/Types/BC_BlockBlue.BC_BlockBlue_C" (`KismetMathLibrary.MakeTransform` _startpos (struct) _returnvalue) "Undefined" "MultiplyWithRoot" null (struct) self null))
    (:`4`
      (`|SpawnActorFromClass` "/Game/Blueprints/Tetris/Types/BC_BlockOrange.BC_BlockOrange_C" (`KismetMathLibrary.MakeTransform` _startpos (struct) _returnvalue) "Undefined" "MultiplyWithRoot" null (struct) self null))
    (:`5`
      (`|SpawnActorFromClass` "/Game/Blueprints/Tetris/Types/BC_BlockOrange_i.BC_BlockOrange_i_C" (`KismetMathLibrary.MakeTransform` _startpos (struct) _returnvalue) "Undefined" "MultiplyWithRoot" null (struct) self null))
    (:`6`
      (`|SpawnActorFromClass` "/Game/Blueprints/Tetris/Types/BP_BlockRed.BP_BlockRed_C" (`KismetMathLibrary.MakeTransform` _startpos (struct) _returnvalue) "Undefined" "MultiplyWithRoot" null (struct) self null))))

(fn `TryLateralMovement`
  (params (MoveAmount :type "Float (double-precision)"))
  (`self.K2_AddActorWorldOffset` (`self.ActualBlock`) (`KismetMathLibrary.MakeVector` 0.0 MoveAmount) false false)
  (for _array_element (`self.K2_GetComponentsByClass` (`self.ActualBlock`) "/Script/Engine.StaticMeshComponent")
    (bind (_outactors _returnvalue) (`KismetSystemLibrary.BoxOverlapActors` (`SceneComponent.K2_GetComponentLocation` _array_element) (15.0 15.0 15.0) (`|MakeArray` "ObjectTypeQuery1" :!type "EObjectTypeQuery Enum")))
    (if _returnvalue
      (`self.K2_AddActorWorldOffset` (`self.ActualBlock`) (`KismetMathLibrary.MakeVector` 0.0 (* MoveAmount -1.0)) false false)
      (break))))

(fn `UserConstructionScript`)