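; Tetris is the container actor that assembles a Tetris game from child actor components for the block spawner, grid and line checker.
; Its Construction Script casts each child actor and passes the grid and line-checker references to BP_BlocksSpawner.
; The event graph holds no active logic, so this Blueprint only wires the parts together.
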(fn `UserConstructionScript`
  (bind _asbp_blocks_spawner (cast `/Game/Blueprints/Tetris/BP_BlocksSpawner` (`ChildActorComponent.ChildActor` (`self.BP_BlocksSpawner`))))
  (bind _asbp_tetris_grid (cast `/Game/Blueprints/Tetris/BP_TetrisGrid` (`ChildActorComponent.ChildActor` (`self.BP_TetrisGrid`))))
  (set `/Game/Blueprints/Tetris/BP_BlocksSpawner.TetrisGrid` _asbp_tetris_grid _asbp_blocks_spawner)
  (bind _asbp_check_lines (cast `/Game/Blueprints/Tetris/BP_CheckLines` (`ChildActorComponent.ChildActor` (`self.BP_CheckLines`))))
  (set `/Game/Blueprints/Tetris/BP_BlocksSpawner.CheckLineActors` _asbp_check_lines _asbp_blocks_spawner))