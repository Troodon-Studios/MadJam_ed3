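; BP_Player is the player Blueprint that sets up mouse-driven combat and spawns a FightingBoard at the CombatSpawn transform on BeginPlay.
; BeginPlay shows the cursor, enables click events and uses Game and UI input, then stores the spawned board.
; Numpad 4–6 keys call the board's Spawner4–6 with "Monster1".
; ActivateMonster maps an index to one of six child-actor BestButton_1 slots and marks it available.
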(event `Key|NumPadOne`
  (params (Key :type "Key Structure")))

(event `Key|NumPadTwo`
  (params (Key :type "Key Structure")))

(event `Key|NumPadThree`
  (params (Key :type "Key Structure")))

(event `Key|NumPadFour`
  (params (Key :type "Key Structure"))
  (:`Pressed`
    (`/Game/Blueprints/Modules/FightingBoard.Spawner4` (`self.FightingBoard`) "Monster1")))

(event `Key|NumPadFive`
  (params (Key :type "Key Structure"))
  (:`Pressed`
    (`/Game/Blueprints/Modules/FightingBoard.Spawner5` (`self.FightingBoard`) "Monster1")))

(event `Key|NumPadSix`
  (params (Key :type "Key Structure"))
  (:`Pressed`
    (`/Game/Blueprints/Modules/FightingBoard.Spawner6` (`self.FightingBoard`) "Monster1")))

(event `self.ReceiveBeginPlay`
  (bind _returnvalue (`GameplayStatics.GetPlayerController` 0))
  (bind (_returnvalue_location _returnvalue_rotation _returnvalue_scale) (`KismetMathLibrary.BreakTransform` (`SceneComponent.K2_GetComponentToWorld` (`self.CombatSpawn`))))
  (set `PlayerController.bShowMouseCursor` true _returnvalue)
  (set `PlayerController.bEnableClickEvents` true _returnvalue)
  (`WidgetBlueprintLibrary.SetInputMode_GameAndUIEx` _returnvalue null "DoNotLock" false true)
  (bind _returnvalue_2 (`|SpawnActorFromClass` "/Game/Blueprints/Modules/FightingBoard.FightingBoard_C" (`KismetMathLibrary.MakeTransform` _returnvalue_location _returnvalue_rotation _returnvalue_scale) "Undefined" "MultiplyWithRoot" null null))
  (set `self.FightingBoard` _returnvalue_2))

(fn `ActivateMonster`
  (params (Int :type Integer))
  (bind _asbest_button_1 (cast `/Game/Blueprints/BestButtons/BestButton_1` (`ChildActorComponent.ChildActor` (select `int` Int :`0` null :`1` (`self.Monster_1`) :`2` (`self.Monster_2`) :`3` (`self.Monster_3`) :`4` (`self.Monster_4`) :`5` (`self.Monster_5`) :`6` (`self.Monster_6`)))))
  (set `/Game/Blueprints/BestButtons/BestButton_1.aviable?` true _asbest_button_1))

(fn `UserConstructionScript`)