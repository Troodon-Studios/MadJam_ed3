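; BestButton_1 is a clickable button actor shown as a skeletal mesh, which the construction script assigns from its Mesh variable.
; Clicking its Box component clears the Aviable flag, and nothing in this Blueprint sets it back.
; Every Tick pushes the Color vector parameter to the mesh materials, overbright white while available and black otherwise.
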(event `self.ReceiveTick`
  (params (DeltaSeconds :type "Float (single-precision)"))
  (`MeshComponent.SetVectorParameterValueOnMaterials` (`self.SM_Monster_01__2_`) "Color" (select `bool` (`self.aviable?`) :`true` (200.0 200.0 200.0) :!type "Vector Structure")))

(event `self.Box.OnClicked`
  (params (TouchedComponent :type "PrimitiveComponent Object Reference") (ButtonPressed :type "Key Structure"))
  (if (`self.aviable?`)
    (set `self.aviable?` false)))

(fn `UserConstructionScript`
  (`SkeletalMeshComponent.SetSkeletalMeshAsset` (`self.SM_Monster_01__2_`) (`self.Mesh`)))