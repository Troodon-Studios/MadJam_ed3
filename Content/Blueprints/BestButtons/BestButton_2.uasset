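; BestButton_2 is a clickable button actor that triggers monster spawning on the fighting board.
; Every tick it drives the monster mesh's "Light" material parameter, blacked out when unavailable.
; Clicking its box while available disables it, then calls Spawner4, Spawner5 and Spawner6 on the first FightingBoard found.
; An integer selects the monster name passed to all three; nothing here re-enables the button.
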(event `self.ReceiveTick`
  (params (DeltaSeconds :type "Float (single-precision)"))
  (`MeshComponent.SetVectorParameterValueOnMaterials` (`self.SM_Monster_01__2_`) "Light" (select `bool` (`self.aviable?`) :`true` (`KismetMathLibrary.Conv_DoubleToVector` (`self.light`)))))

(event `self.Box.OnClicked`
  (params (TouchedComponent :type "PrimitiveComponent Object Reference") (ButtonPressed :type "Key Structure"))
  (bind _returnvalue (select `int` (`self.int`) :`0` "Monster1" :`1` "Monster1" :`2` "Monster2" :`3` "Monster3" :`4` "Monster4" :`5` "Monster5" :`6` "Monster6" :!type "Name"))
  (if (`self.aviable?`)
    (set `self.aviable?` false)
    (bind _outactors (`GameplayStatics.GetAllActorsOfClass` "/Game/Blueprints/Modules/FightingBoard.FightingBoard_C"))
    (bind _output (`|GetArrayItem` _outactors))
    (`/Game/Blueprints/Modules/FightingBoard.Spawner4` _output _returnvalue)
    (`/Game/Blueprints/Modules/FightingBoard.Spawner5` _output _returnvalue)
    (`/Game/Blueprints/Modules/FightingBoard.Spawner6` _output _returnvalue)))

(fn `UserConstructionScript`)